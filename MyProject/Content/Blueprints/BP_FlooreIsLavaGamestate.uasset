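; Game state for a floor-is-lava first-person game, tracking the run timer, coins, checkpoint and the player's height above the lava.
; BeginPlay counts coins in the level, caches the player and first lava actor, and records the spawn transform.
; StartGame waits three seconds, once, before enabling timing.
; Tick then accumulates rounded time and recomputes the vertical player-to-lava distance, while other events update coin counts and saved checkpoint.
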(event `Count Coins`
  (bind _outactors (`GameplayStatics.GetAllActorsOfClass` "/Game/Blueprints/Obstacles/BP_Coin.BP_Coin_C"))
  (set `self.Coins Left` (`KismetArrayLibrary.Array_Length` _outactors)))

(event `Start Game`
  (`/Engine/EditorBlueprintResources/StandardMacros.DoOnce` false
    (:`Completed`
      (`KismetSystemLibrary.Delay` 3.0)
      (set `self.Time Started?` true))))

(event `self.ReceiveBeginPlay`
  (`|ExecutionSequence`
    (:`then_0`
      (set `self.Time Started?` false)
      (`self.Count Coins`)
      (`WidgetBlueprintLibrary.SetInputMode_GameOnly` (`GameplayStatics.GetPlayerController` 0))
      (bind _asbp_first_person_character (cast `/Game/FirstPerson/Blueprints/BP_FirstPersonCharacter` (`GameplayStatics.GetPlayerPawn` 0)))
      (set `self.PlayerRef` _asbp_first_person_character)
      (bind _outactors (`GameplayStatics.GetAllActorsOfClass` "/Game/Blueprints/BP_Lava.BP_Lava_C"))
      (set `self.LavaRef` (`|GetArrayItem` _outactors)))
    (:`then_1`
      (set `self.Spawn Point` (`self.GetTransform` (`GameplayStatics.GetPlayerPawn` 0))))))

(event `self.ReceiveTick`
  (params (DeltaSeconds :type "Float (single-precision)"))
  (if (`self.Time Started?`)
    (`self.Increase Timer` DeltaSeconds)
    (`self.Calculate Distance`)))

(event `Increase Timer`
  (params (`Time to Add` :type "Float (double-precision)"))
  (bind _output_get (set `self.Total Time` (+ `Time to Add` (`self.Total Time`))))
  (set `self.Rounded Time` (`KismetStringLibrary.Conv_IntToString` (`KismetMathLibrary.Round` _output_get))))

(event `Add Coins`
  (set `self.Coins Collected` (+ (`self.Coins Collected`) 1)))

(event `Remove Coin From Total`
  (set `self.Coins Left` (- (`self.Coins Left`) 1)))

(event `Set Checkpoint Number`
  (params (Checkpoint :type Integer))
  (set `self.Saved Checkpoint` Checkpoint))

(event `Calculate Distance`
  (bind _asbp_first_person_character (cast `/Game/FirstPerson/Blueprints/BP_FirstPersonCharacter` (`GameplayStatics.GetPlayerPawn` 0)))
  (bind _output_get (set `self.Distance` (- (.z (.location (`self.GetTransform` _asbp_first_person_character))) (.z (.location (`self.GetTransform` (`self.LavaRef`)))))))
  (set `self.Distance Rounded` (`KismetMathLibrary.Round` (/ _output_get 100.0))))

(fn `UserConstructionScript`)