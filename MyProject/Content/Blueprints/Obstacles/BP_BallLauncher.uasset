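; BP_BallLauncher is an obstacle that repeatedly fires BP_Ball actors from its Arrow component's location and rotation.
; Tick accumulates delta time in a counter, compares it to a random threshold re-rolled every frame, then resets and calls FireBall.
; FireBall spawns the ball and plays a very quiet, attenuated grenade launcher sound at the actor.
; A looping timer call to FireBall is left unconnected.
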(event `self.ReceiveTick`
  (params (DeltaSeconds :type "Float (single-precision)"))
  (bind _output_get (set `self.counter` (+ (`self.counter`) DeltaSeconds)))
  (if (> _output_get (`KismetMathLibrary.RandomFloatInRange` 1.5 3.0))
    (set `self.counter` 0.0)
    (`self.FireBall`)))

(event `self.ReceiveBeginPlay`
  (set `self.counter` 0.0))

(event `FireBall`
  (bind _arrow (`self.Arrow`))
  (`|SpawnActorFromClass` "/Game/Blueprints/BP_Ball.BP_Ball_C" (`KismetMathLibrary.MakeTransform` (`SceneComponent.K2_GetComponentLocation` _arrow) (`SceneComponent.K2_GetComponentRotation` _arrow)) "Undefined" "MultiplyWithRoot" null null)
  (`GameplayStatics.PlaySoundAtLocation` "/Game/Blueprints/grenade-launcher-106342.grenade-launcher-106342" (`self.K2_GetActorLocation`) (`SceneComponent.K2_GetComponentRotation` (`self.Arrow`)) 0.001 1.0 0.0 "/Game/Blueprints/BallSound.BallSound" null null null))

(fn `UserConstructionScript`)