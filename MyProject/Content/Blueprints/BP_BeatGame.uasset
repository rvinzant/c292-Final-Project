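; BP_BeatGame is a goal trigger that ends the floor-is-lava game with a win screen once enough coins are collected.
; Overlapping its CollisionBox checks the game state's coin count.
; At the threshold, after a short delay, a player-pawn overlap shows WBP_WinScreen, enables the cursor and UI-only input, and pauses the game.
; Below it, any overlapping actor causes WBP_Instructions2 to appear.
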(event `self.Collision Box.OnComponentBeginOverlap`
  (params (OverlappedComponent :type "PrimitiveComponent Object Reference") (OtherActor :type "Actor Object Reference") (OtherComp :type "PrimitiveComponent Object Reference") (OtherBodyIndex :type Integer) (bFromSweep :type Boolean) (SweepResult :type "HitResult Structure (by ref)"))
  (bind _asbp_floore_is_lava_gamestate (cast `/Game/Blueprints/BP_FlooreIsLavaGamestate` (`GameplayStatics.GetGameState`)))
  (if (>= (`/Game/Blueprints/BP_FlooreIsLavaGamestate.Coins Collected` _asbp_floore_is_lava_gamestate) 10)
    (`KismetSystemLibrary.Delay` 0.5)
    (if (== OtherActor (`GameplayStatics.GetPlayerPawn` 0))
      (set `PlayerController.bShowMouseCursor` true (`GameplayStatics.GetPlayerController` 0))
      (bind _returnvalue (`|CreateWidget` "/Game/Blueprints/WBP_WinScreen.WBP_WinScreen_C"))
      (`UserWidget.AddToViewport` _returnvalue 0)
      (`WidgetBlueprintLibrary.SetInputMode_UIOnlyEx` (`GameplayStatics.GetPlayerController` 0) null)
      (`GameplayStatics.SetGamePaused` true))
    (else
      (bind _returnvalue_2 (`|CreateWidget` "/Game/Blueprints/WBP_Instructions2.WBP_Instructions2_C"))
      (`UserWidget.AddToViewport` _returnvalue_2 0))))

(fn `UserConstructionScript`)