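; BP_FallingPlatform is a platform that drops out from under whatever touches it by disappearing, then returns.
; A Box overlap triggers a DoOnce that, after a short delay, hides the Cube and disables its collision.
; After a longer delay it restores visibility and collision and resets the DoOnce for reuse.
; Actor overlap also saves the transform to OriginalLocation, but nothing here reads it or moves the platform.
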(event `self.ReceiveActorBeginOverlap`
  (params (OtherActor :type "Actor Object Reference"))
  (set `self.Original Location` (`self.GetTransform`)))

(event `self.Box.OnComponentBeginOverlap`
  (params (OverlappedComponent :type "PrimitiveComponent Object Reference") (OtherActor :type "Actor Object Reference") (OtherComp :type "PrimitiveComponent Object Reference") (OtherBodyIndex :type Integer) (bFromSweep :type Boolean) (SweepResult :type "HitResult Structure (by ref)"))
  (`/Engine/EditorBlueprintResources/StandardMacros.DoOnce` false :!label _label
    (:`Completed`
      (`KismetSystemLibrary.Delay` 0.5)
      (`SceneComponent.SetVisibility` (`self.Cube`) false false)
      (`PrimitiveComponent.SetCollisionEnabled` (`self.Cube`) "NoCollision")
      (`KismetSystemLibrary.Delay` 3.0)
      (`SceneComponent.SetVisibility` (`self.Cube`) true false)
      (`PrimitiveComponent.SetCollisionEnabled` (`self.Cube`) "QueryAndPhysics")
      (goto _label :!via `Reset`))))

(fn `UserConstructionScript`)