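; BP_StartButton is an interactable button that starts the Floor is Lava game.
; On the first Interact only, it nudges the SMClock component inward along local X and plays a start sound.
; It then calls StartGame on BP_FlooreIsLavaGamestate, shows and starts a WBP_Countdown widget for player 0, and sets every BP_Lava actor active.
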(event `/Game/Blueprints/BPI_Interactable.Interact`
  (params (`Player Ref` :type "/Game/FirstPerson/Blueprints/BP_FirstPersonCharacter Object Reference"))
  (`/Engine/EditorBlueprintResources/StandardMacros.DoOnce` false
    (:`Completed`
      (`SceneComponent.K2_AddRelativeLocation` (`self.SM_Clock`) (-6.0 0.0 0.0) false false)
      (`GameplayStatics.PlaySoundAtLocation` "/Game/Blueprints/Sounds/Start_Sound.Start_Sound" (`self.K2_GetActorLocation`) (struct) 1.0 1.0 0.0 null null null null)
      (bind _asbp_floore_is_lava_gamestate (cast `/Game/Blueprints/BP_FlooreIsLavaGamestate` (`GameplayStatics.GetGameState`)))
      (`/Game/Blueprints/BP_FlooreIsLavaGamestate.Start Game` _asbp_floore_is_lava_gamestate)
      (bind _returnvalue (`|CreateWidget` "/Game/Blueprints/UI/WBP_Countdown.WBP_Countdown_C" (`GameplayStatics.GetPlayerController` 0)))
      (`UserWidget.AddToViewport` _returnvalue 0)
      (`/Game/Blueprints/UI/WBP_Countdown.Start Countdown` _returnvalue)
      (bind _outactors (`GameplayStatics.GetAllActorsOfClass` "/Game/Blueprints/BP_Lava.BP_Lava_C"))
      (for _array_element _outactors
        (set `/Game/Blueprints/BP_Lava.IsActive?` true _array_element)))))

(fn `UserConstructionScript`)