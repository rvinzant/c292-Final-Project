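; BP_CheckPoint is a checkpoint obstacle for the floor-is-lava mode that records player progress.
; Its box overlap passes a DoOnce before the player-pawn check, so the first overlap by any actor uses it up.
; For the player, it saves the current lava location, its spawn point transform and checkpoint number to BP_FlooreIsLavaGamestate, then plays a sound.
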(event `self.Box.OnComponentBeginOverlap`
  (params (OverlappedComponent :type "PrimitiveComponent Object Reference") (OtherActor :type "Actor Object Reference") (OtherComp :type "PrimitiveComponent Object Reference") (OtherBodyIndex :type Integer) (bFromSweep :type Boolean) (SweepResult :type "HitResult Structure (by ref)"))
  (`/Engine/EditorBlueprintResources/StandardMacros.DoOnce` false
    (:`Completed`
      (if (== OtherActor (`GameplayStatics.GetPlayerPawn` 0))
        (bind _asbp_floore_is_lava_gamestate (cast `/Game/Blueprints/BP_FlooreIsLavaGamestate` (`GameplayStatics.GetGameState`)))
        (set `/Game/Blueprints/BP_FlooreIsLavaGamestate.Lava` (`self.K2_GetActorLocation` (`/Game/Blueprints/BP_FlooreIsLavaGamestate.LavaRef` _asbp_floore_is_lava_gamestate)) _asbp_floore_is_lava_gamestate)
        (set `/Game/Blueprints/BP_FlooreIsLavaGamestate.Spawn Point` (`SceneComponent.K2_GetComponentToWorld` (`self.SpawnPoint`)) _asbp_floore_is_lava_gamestate)
        (`/Game/Blueprints/BP_FlooreIsLavaGamestate.Set Checkpoint Number` _asbp_floore_is_lava_gamestate (`self.CheckpointNumber`))
        (`GameplayStatics.PlaySoundAtLocation` "/Game/Blueprints/Sounds/CheckpointSound.CheckpointSound" (`self.K2_GetActorLocation`) (struct) 1.0 1.0 0.0 null null null null)))))

(fn `UserConstructionScript`)