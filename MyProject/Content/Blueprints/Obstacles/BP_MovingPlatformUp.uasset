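; BP_MovingPlatformUp is an obstacle platform that moves up and down continuously from where it is placed.
; On BeginPlay it stores its location and a point 200 units above, then plays the PlatformMovement timeline to lerp between them without sweeping.
; A FlipFlop on Finished alternates Reverse and Play to loop the motion.
; Speed multiplies the lerp alpha, so it scales travel distance rather than timeline rate.
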(event `self.ReceiveBeginPlay`
  (bind (_start_x _start_y _start_z) (`KismetMathLibrary.BreakVector` (`self.Start`)))
  (set `self.Start` (`self.K2_GetActorLocation`))
  (set `self.End` (`KismetMathLibrary.MakeVector` _start_x _start_y (+ _start_z 200.0)))
  (bind (_direction _movealpha) (`Timeline|PlatformMovement` :!label _label)
    (:`Update`
      (`self.K2_SetActorLocation` (`KismetMathLibrary.VLerp` (`self.Start`) (`self.End`) (* _movealpha (`self.speed`)))))
    (:`Finished`
      (`/Engine/EditorBlueprintResources/StandardMacros.FlipFlop`
        (:`A`
          (goto _label :!via `Reverse`))
        (:`B`
          (goto _label))))))

(event `self.ReceiveTick`
  (params (DeltaSeconds :type "Float (single-precision)")))

(fn `UserConstructionScript`)